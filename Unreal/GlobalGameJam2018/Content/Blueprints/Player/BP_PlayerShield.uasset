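; BP_PlayerShield is a one-hit player shield that knocks back incoming Robbert_Objects actors.
; On overlap, it reacts only when the object's speed exceeds MinimumTriggerForce.
; It reverses the object's physics velocity, scaled by ForceMultiplier, then flags itself broken, hides and destroys itself.
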(event `self.ReceiveTick`
  (params (DeltaSeconds :type "Float (single-precision)")))

(event `self.ReceiveActorBeginOverlap`
  (params (OtherActor :type "Actor Object Reference"))
  (bind _asrobbert_objects (cast `/Game/Robbert_Objects` OtherActor))
  (bind _returnvalue (`self.GetVelocity` _asrobbert_objects))
  (if (> (`KismetMathLibrary.VSize` _returnvalue) (`self.MinimumTriggerForce`))
    (`PrimitiveComponent.SetPhysicsLinearVelocity` (`/Game/Robbert_Objects.StaticMesh` _asrobbert_objects) (* (* _returnvalue -1.0) (`self.ForceMultiplier`)) false "None")
    (set `self.IsBroken` true)
    (`self.SetActorHiddenInGame` true)
    (`self.K2_DestroyActor`)))

(fn `UserConstructionScript`)