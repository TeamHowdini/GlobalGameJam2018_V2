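; Per-player menu pawn that handles joining, leaving and the start countdown before the game level opens.
; Start and Back events set this PlayerID's ready state and selection image, play a sound and notify BP_MenuGameMode, which is also told when Start is released.
; Tick raises or drains the menu widget's start percentage based on the game mode's readiness flag, opening the level when full.
; The Menu_Button input quits the game.
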(event `self.ReceiveBeginPlay`
  (bind _asbp_menu_game_mode (cast `/Game/Blueprints/Core/Gamemodes/BP_MenuGameMode` (`GameplayStatics.GetGameMode`)))
  (set `self.MenuGameMode` _asbp_menu_game_mode))

(event `self.ReceiveTick`
  (params (DeltaSeconds :type "Float (single-precision)"))
  (bind _menugamemode (`self.MenuGameMode`))
  (bind _menuwidgetref (`/Game/Blueprints/Core/Gamemodes/BP_MenuGameMode.MenuWidgetRef` _menugamemode))
  (bind _startpercentage (`/Game/UI/Menus/Menu_Widget.StartPercentage` _menuwidgetref))
  (if (`/Game/Blueprints/Core/Gamemodes/BP_MenuGameMode.IncreateReadiness` _menugamemode)
    (if (>= _startpercentage 1.0)
      (set `/Game/Blueprints/Core/Gamemodes/BP_MenuGameMode.IncreateReadiness` false _menugamemode)
      (`/Game/Blueprints/Core/Gamemodes/BP_MenuGameMode.OpenGameLevel` _menugamemode)
      (else
        (set `/Game/UI/Menus/Menu_Widget.StartPercentage` (`KismetMathLibrary.FClamp` (+ DeltaSeconds _startpercentage)) _menuwidgetref)))
    (else
      (set `/Game/UI/Menus/Menu_Widget.StartPercentage` (`KismetMathLibrary.FClamp` (- _startpercentage DeltaSeconds)) _menuwidgetref))))

(event `self.StartPressed`
  (bind _playerid (`self.playerID`))
  (bind _menugamemode (`self.MenuGameMode`))
  (`GameplayStatics.PlaySound2D` "/Game/Assets/Sounds/S_SFX_Cues/SC_SFX_UI_Menu_PlayerJoin.SC_SFX_UI_Menu_PlayerJoin" 1.0 1.0 0.0 null null)
  (`/Game/Blueprints/Core/Gamemodes/BP_MenuGameMode.SetIsPlayerReady` _menugamemode _playerid true)
  (`/Game/UI/Menus/Menu_Widget.SetPlayerSelectionImage` (`/Game/Blueprints/Core/Gamemodes/BP_MenuGameMode.MenuWidgetRef` _menugamemode) true _playerid)
  (`/Game/Blueprints/Core/Gamemodes/BP_MenuGameMode.PlayerPressedStart` _menugamemode))

(event `self.EndPressed`
  (`/Game/Blueprints/Core/Gamemodes/BP_MenuGameMode.PlayerReleasedStart` (`self.MenuGameMode`)))

(event `self.BackPressed`
  (bind _playerid (`self.playerID`))
  (bind _menugamemode (`self.MenuGameMode`))
  (`GameplayStatics.PlaySound2D` "/Game/Assets/Sounds/S_SFX_Cues/SC_SFX_UI_Menu_PlayerJoin.SC_SFX_UI_Menu_PlayerJoin" 1.0 1.0 0.0 null null)
  (`/Game/Blueprints/Core/Gamemodes/BP_MenuGameMode.SetIsPlayerReady` _menugamemode _playerid false)
  (`/Game/UI/Menus/Menu_Widget.SetPlayerSelectionImage` (`/Game/Blueprints/Core/Gamemodes/BP_MenuGameMode.MenuWidgetRef` _menugamemode) false _playerid)
  (`/Game/Blueprints/Core/Gamemodes/BP_MenuGameMode.PlayerPressedBack` _menugamemode))

(event `InputAction|Menu_Button`
  (params (Key :type "Key Structure"))
  (:`Pressed`
    (`KismetSystemLibrary.QuitGame` null "Quit")))

(fn `UserConstructionScript`)