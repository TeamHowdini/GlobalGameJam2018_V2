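; Player character with telekinesis that pulls, orbits and flings ObjectBase actors.
; Pull floats objects in range within PowerLevel, which grows over time; Tick eases them into orbit, locking those in front to an aim point.
; Push launches held objects along the facing direction; releasing Pull drops them.
; Fast hits from objects the player doesn't own cause weight-based damage, ragdolling at zero health; M toggles mouse facing.
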(event `self.ReceiveBeginPlay`)

(event `InputAction|Pull`
  (params (Key :type "Key Structure"))
  (bind _gravitywell (`self.GravityWell`))
  (bind _gravityparticleeffect (`self.GravityParticleEffect`))
  (bind _lockedobjects (`self.LockedObjects`))
  (bind _activatedobjects (`self.ActivatedObjects`))
  (:`Pressed`
    (`SceneComponent.SetVisibility` _gravitywell true false)
    (`ActorComponent.Activate` _gravityparticleeffect false)
    (bind _returnvalue (`GameplayStatics.SpawnSoundAttached` "/Game/Assets/Sounds/S_SFX_Cues/SC_SFX_Player_Telekenesis_ActiveLOOP.SC_SFX_Player_Telekenesis_ActiveLOOP" (`self.Mesh`)))
    (`AudioComponent.Play` _returnvalue 0.0)
    (set `self.Pulsing Sound` _returnvalue)
    (`GameplayStatics.PlaySoundAtLocation` "/Game/Assets/Sounds/S_SFX_Cues/SC_SFX_Player_Telekenesis_Pull.SC_SFX_Player_Telekenesis_Pull" (`self.K2_GetActorLocation`))
    (set `self.IsPulling` true)
    (bind _outactors (`GameplayStatics.GetAllActorsOfClass` "/Game/Blueprints/Objects/ObjectBase.ObjectBase_C"))
    (for _array_element _outactors
      (if (< (`KismetMathLibrary.VSize` (- (`/Game/Blueprints/Objects/ObjectBase.GetLocation` _array_element) (`self.K2_GetActorLocation`))) (`self.PullRange`))
        (if (>= (`self.PowerLevel`) (`/Game/Blueprints/Objects/ObjectBase.WeightLevel` _array_element))
          (`KismetArrayLibrary.Array_Add` (`self.ActivatedObjects`) _array_element)
          (`/Game/Blueprints/Objects/ObjectBase.Float` _array_element)))))
  (:`Released`
    (`SceneComponent.SetVisibility` _gravitywell false false)
    (`ActorComponent.Deactivate` _gravityparticleeffect)
    (`AudioComponent.FadeOut` (`self.Pulsing Sound`) 0.5 0.0)
    (`|ExecutionSequence`
      (:`then_0`
        (set `self.IsPulling` false)
        (for _array_element_2 _activatedobjects
          (`/Game/Blueprints/Objects/ObjectBase.StopFloat` _array_element_2))
        (`KismetArrayLibrary.Array_Clear` _activatedobjects))
      (:`then_1`
        (for _array_element_3 _lockedobjects
          (`/Game/Blueprints/Objects/ObjectBase.StopFloat` _array_element_3))
        (`KismetArrayLibrary.Array_Clear` _lockedobjects)))))

(event `self.ReceiveTick`
  (params (DeltaSeconds :type "Float (single-precision)"))
  (bind _returnvalue (`self.K2_GetActorLocation`))
  (bind _shieldcenter (`self.ShieldCenter`))
  (bind (_returnvalue_x _returnvalue_y) (`KismetMathLibrary.BreakVector2D` (- (`KismetMathLibrary.MakeVector2D` (`self.GetInputAxisKeyValue`) (`self.GetInputAxisKeyValue`)) (/ (`WidgetLayoutLibrary.GetViewportSize`) 2.0))))
  (`|ExecutionSequence`
    (:`then_0`
      ;[1 1 1] Handle Pulling Of Objects
      (for _array_element (`self.ActivatedObjects`)
        (bind _returnvalue_2 (- (`self.ObjectFloatingPosition`) (`/Game/Blueprints/Objects/ObjectBase.GetLocation` _array_element)))
        (`/Game/Blueprints/Objects/ObjectBase.AddForceCustom` _array_element (* (`KismetMathLibrary.Normal` _returnvalue_2) (* (`KismetMathLibrary.VSize` _returnvalue_2) (`self.LinearForceMultiplier`))))
        (bind _newparam (`/Game/Blueprints/Objects/ObjectBase.GetLocation` _array_element))
        (`/Game/Blueprints/Objects/ObjectBase.SetLocation` _array_element (+ _newparam (* (- (+ _returnvalue (* (`KismetMathLibrary.Normal` (- _newparam _returnvalue)) (`self.OrbitRange`))) _newparam) 0.2)) false)
        (if (> (`KismetMathLibrary.Dot_VectorVector` (`KismetMathLibrary.Normal` (- _newparam _returnvalue)) (`self.GetActorForwardVector`)) (`self.FloatLockBias`))
          (`KismetArrayLibrary.Array_Add` (`self.LockedObjects`) _array_element)
          (`KismetArrayLibrary.Array_RemoveItem` (`self.ActivatedObjects`) _array_element)
          (`KismetSystemLibrary.PrintString` "LOCKED!"))))
    (:`then_1`
      (bind _output_get (set `self.ObjectFloatingPosition` (+ (`self.K2_GetActorLocation`) (* (`self.AimRotation`) (`self.OrbitRange`))))))
    (:`then_2`
      ;[1 1 1] Handle Locked Objects
      (for _array_element_2 (`self.LockedObjects`)
        (bind _newparam_2 (`/Game/Blueprints/Objects/ObjectBase.GetLocation` _array_element_2))
        (`/Game/Blueprints/Objects/ObjectBase.SetLocation` _array_element_2 (+ _newparam_2 (`KismetMathLibrary.ClampVectorSize` (* (- (`self.ObjectFloatingPosition`) _newparam_2) DeltaSeconds) (* (`self.MaxObjectSpeedScuffed`) -1.0) (`self.MaxObjectSpeedScuffed`))) false)
        (set `/Game/Blueprints/Objects/ObjectBase.OwnerPlayer` self _array_element_2)))
    (:`then_3`
      (if (`self.MouseMode`)
        (`self.K2_SetActorRotation` (`KismetMathLibrary.MakeRotFromX` (`KismetMathLibrary.MakeVector` _returnvalue_x _returnvalue_y)))
        (set `PlayerController.bShowMouseCursor` true (`GameplayStatics.GetPlayerController` 0))))
    (:`then_4`
      (set `self.PowerLevel` (+ (`self.PowerLevel`) DeltaSeconds)))
    (:`then_5`
      (`SceneComponent.K2_SetWorldRotation` _shieldcenter (`KismetMathLibrary.MakeRotator` (.roll (`SceneComponent.K2_GetComponentRotation` _shieldcenter)) (.pitch (`SceneComponent.K2_GetComponentRotation` _shieldcenter)) (+ (.yaw (`SceneComponent.K2_GetComponentRotation` _shieldcenter)) (* DeltaSeconds (`self.RotationFactor`)))) false false))))

(event `Key|M`
  (params (Key :type "Key Structure"))
  (:`Pressed`
    (set `self.MouseMode` (not (`self.MouseMode`)))))

(event `InputAction|Push`
  (params (Key :type "Key Structure"))
  (bind _activatedobjects (`self.ActivatedObjects`))
  (:`Pressed`
    (`ActorComponent.Activate` (`self.PushParticleEffect`) false)
    (`GameplayStatics.PlaySoundAtLocation` "/Game/Assets/Sounds/S_SFX_Cues/SC_SFX_Player_Telekenesis_Push.SC_SFX_Player_Telekenesis_Push" (`self.K2_GetActorLocation`))
    (`|ExecutionSequence`
      (:`then_0`
        (for _array_element (`self.LockedObjects`)
          (`/Game/Blueprints/Objects/ObjectBase.AddImpulse` _array_element (* (`self.GetActorForwardVector`) (`self.PushImpulseMult`)))
          (`/Game/Blueprints/Objects/ObjectBase.StopFloat` _array_element))
        (`KismetArrayLibrary.Array_Clear` (`self.LockedObjects`)))
      (:`then_1`
        (for _array_element_2 _activatedobjects
          (`/Game/Blueprints/Objects/ObjectBase.AddImpulse` _array_element_2 (* (`self.GetActorForwardVector`) (`self.PushImpulseMult`)))
          (`/Game/Blueprints/Objects/ObjectBase.StopFloat` _array_element_2))
        (`KismetArrayLibrary.Array_Clear` _activatedobjects)))))

(event `self.ReceiveHit`
  (params (MyComp :type "PrimitiveComponent Object Reference") (Other :type "Actor Object Reference") (OtherComp :type "PrimitiveComponent Object Reference") (bSelfMoved :type Boolean) (HitLocation :type "Vector Structure") (HitNormal :type "Vector Structure") (NormalImpulse :type "Vector Structure") (Hit :type "HitResult Structure (by ref)"))
  (bind _mesh (`self.Mesh`))
  (bind _asobject_base (cast `/Game/Blueprints/Objects/ObjectBase` (`ActorComponent.GetOwner` OtherComp)))
  (if (not (== (`/Game/Blueprints/Objects/ObjectBase.OwnerPlayer` _asobject_base) self))
    (bind _newparam (`/Game/Blueprints/Objects/ObjectBase.GetVel` _asobject_base))
    (if (> (`KismetMathLibrary.VSize` _newparam) (`self.MinDamageVelocity`))
      (`/Game/Blueprints/Objects/ObjectBase.AddImpulse` _asobject_base (* _newparam -0.3))
      (if (`self.CanTakeDamage`)
        (bind _returnvalue (`self.DecrementHealth` (`KismetMathLibrary.FTrunc` (* (`/Game/Blueprints/Objects/ObjectBase.WeightLevel` _asobject_base) 4.0))))
        (set `self.CanTakeDamage` false)
        (`KismetSystemLibrary.K2_SetTimer` null "CanTakeDamage" 0.3)
        (if (<= _returnvalue 0)
          (`PrimitiveComponent.SetSimulatePhysics` _mesh true)
          (`PrimitiveComponent.SetCollisionEnabled` _mesh "QueryAndPhysics")
          (`self.DetachFromControllerPendingDestroy`)
          (`ActorComponent.K2_DestroyComponent` (`self.ShieldCenter`))
          (`PlayerController.ClientStartCameraShake` :`self` (`GameplayStatics.GetPlayerController` 0) :`Shake` "/Game/Blueprints/Camera/BP_ScreenShake.BP_ScreenShake_C" :`Scale` 1.5))))))

(fn `EnableDamage`
  (set `self.CanTakeDamage` true))

(fn `UserConstructionScript`)