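; Main game mode that ends a match when fewer than two player characters remain alive.
; Until victory is flagged, Tick gathers every BP_PlayerCharacter and counts those with at least 1 health.
; When the count drops below two, it sets the flag, plays victory music and shows the victory widget after calling its SetColor.
; A five-second timer then opens the menu level.
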(event `self.ReceiveTick`
  (params (DeltaSeconds :type "Float (single-precision)"))
  (if (not (`self.Victory`))
    (set `self.PlayersAlive` 0)
    (bind _outactors (`GameplayStatics.GetAllActorsOfClass` "/Game/Blueprints/Player/BP_PlayerCharacter.BP_PlayerCharacter_C"))
    (for _array_element _outactors
      (bind _returnvalue (`PlayerCharacter.GetHealth` _array_element))
      (if (not (< _returnvalue 1))
        (`/Engine/EditorBlueprintResources/StandardMacros.IncrementInt` (`self.PlayersAlive`))))
    (if (< (`self.PlayersAlive`) 2)
      (`GameplayStatics.PlaySound2D` "/Game/Assets/Music/SC_Music_Victory.SC_Music_Victory")
      (set `self.Victory` true)
      (`KismetSystemLibrary.K2_SetTimer` null "FuckOffBackToMenu" 5.0)
      (bind _returnvalue_2 (`|CreateWidget` "/Game/UI/HUD/VictoryWidget.VictoryWidget_C"))
      (`/Game/UI/HUD/VictoryWidget.SetColor` :`self` _returnvalue_2)
      (`UserWidget.AddToViewport` _returnvalue_2 0))))

(fn `FuckOffBackToMenu`
  (`GameplayStatics.OpenLevel` "Menu_Level"))

(fn `UserConstructionScript`)