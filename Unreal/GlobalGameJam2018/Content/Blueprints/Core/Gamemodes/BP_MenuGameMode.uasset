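; Game mode for the main menu, handling local multiplayer setup, player readiness and the game level launch.
; BeginPlay starts menu music, shows the menu widget and creates three extra local players, storing them in the game instance and assigning pawn IDs.
; Start/Back events toggle a readiness-increase flag, while index-based helpers access four ready flags.
; OpenGameLevel adds ready players to the game instance's connected count, then opens the level by name.
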(event `self.ReceiveBeginPlay`
  (bind _asbp_main_game_instance (cast `/Game/Blueprints/Core/BP_MainGameInstance` (`GameplayStatics.GetGameInstance`)))
  (set `self.MainGameInstance` _asbp_main_game_instance)
  (`GameplayStatics.PlaySound2D` "/Game/Assets/Music/SC_Music_menu.SC_Music_menu" 1.0 1.0 0.0 null null)
  (bind _returnvalue (`|CreateWidget` "/Game/UI/Menus/Menu_Widget.Menu_Widget_C"))
  (bind _output_get (set `self.MenuWidgetRef` _returnvalue))
  (`UserWidget.AddToViewport` _output_get 0)
  (for _index (range 1 4)
    (bind _returnvalue_2 (`GameplayStatics.CreatePlayer` _index))
    (bind _returnvalue_3 (`KismetArrayLibrary.Array_AddUnique` (`/Game/Blueprints/Core/BP_MainGameInstance.ConnectedPlayers` (`self.MainGameInstance`)) _returnvalue_2))
    (bind _asbp_menu_pawn (cast `/Game/Blueprints/Player/BP_MenuPawn` (`Controller.K2_GetPawn` _returnvalue_2)))
    (set `/Game/Blueprints/Player/BP_MenuPawn.PlayerID` _returnvalue_3 _asbp_menu_pawn)))

(event `self.ReceiveTick`
  (params (DeltaSeconds :type "Float (single-precision)")))

(event `OpenGameLevel`
  (for (_ _array_index) (`/Game/Blueprints/Core/BP_MainGameInstance.ConnectedPlayers` (`self.MainGameInstance`))
    (bind _bisready (`self.GetIsPlayerReady` _array_index))
    (if _bisready
      (bind _asbp_main_game_instance (cast `/Game/Blueprints/Core/BP_MainGameInstance` (`GameplayStatics.GetGameInstance`)))
      (bind _numberofconnectedplayers (`/Game/Blueprints/Core/BP_MainGameInstance.NumberOfConnectedPlayers` _asbp_main_game_instance))
      (`/Engine/EditorBlueprintResources/StandardMacros.IncrementInt` _numberofconnectedplayers
        (:`  `
          (`KismetSystemLibrary.PrintString` (`KismetStringLibrary.Conv_IntToString` _numberofconnectedplayers))))))
  (`GameplayStatics.OpenLevel` (`self.LevelName`)))

(event `PlayerPressedStart`
  (set `self.IncreateReadiness` true))

(event `PlayerReleasedStart`
  (set `self.IncreateReadiness` false))

(event `PlayerPressedBack`
  (set `self.IncreateReadiness` false))

(fn `GetIsPlayerReady`
  (params (Index :type Integer))
  (returns (bIsReady :type Boolean))
  (switch `int` Index
    (:`0`
      (return (`self.bIsPlayer1Ready`)))
    (:`1`
      (return (`self.bIsPlayer2Ready`)))
    (:`2`
      (return (`self.bIsPlayer3Ready`)))
    (:`3`
      (return (`self.bIsPlayer4Ready`)))))

(fn `SetIsPlayerReady`
  (params (Index :type Integer) (Condition :type Boolean))
  (switch `int` Index
    (:`0`
      (set `self.bIsPlayer1Ready` Condition))
    (:`1`
      (set `self.bIsPlayer2Ready` Condition))
    (:`2`
      (set `self.bIsPlayer3Ready` Condition))
    (:`3`
      (set `self.bIsPlayer4Ready` Condition))))

(fn `UserConstructionScript`)