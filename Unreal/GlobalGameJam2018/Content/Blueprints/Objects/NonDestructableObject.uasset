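; Physics-driven world object that can float, extending a parent class that defines the float, force and location interface.
; Float turns off gravity on the static mesh and shows a Plane component, and StopFloat reverses both.
; While floating, Tick teleports the Plane to follow the mesh at the offset cached on BeginPlay.
; Force, impulse and location calls act directly on the mesh, with impulses applied as velocity changes.
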(event `self.ReceiveBeginPlay`
  (`parent.ReceiveBeginPlay`)
  (set `self.PlaneOffset` (- (`SceneComponent.K2_GetComponentLocation` (`self.Plane`)) (`SceneComponent.K2_GetComponentLocation` (`self.StaticMesh`)))))

(event `self.ReceiveTick`
  (params (DeltaSeconds :type "Float (single-precision)"))
  (`parent.ReceiveTick` DeltaSeconds)
  (if (`self.IsFloating`)
    (`SceneComponent.K2_SetWorldLocationAndRotation` :`self` (`self.Plane`) :`NewLocation` (+ (`SceneComponent.K2_GetComponentLocation` (`self.StaticMesh`)) (`self.PlaneOffset`)) :`bTeleport` true)))

(event `self.Float`
  (`parent.Float`)
  (`PrimitiveComponent.SetEnableGravity` (`self.StaticMesh`) false)
  (`SceneComponent.SetVisibility` (`self.Plane`) true false))

(event `self.StopFloat`
  (`parent.StopFloat`)
  (`PrimitiveComponent.SetEnableGravity` (`self.StaticMesh`) true)
  (`SceneComponent.SetVisibility` (`self.Plane`) false false))

(event `self.AddForceCustom`
  (params (Force :type "Vector Structure"))
  (`PrimitiveComponent.AddForce` (`self.StaticMesh`) Force "None" false))

(event `self.SetLocation`
  (params (Location :type "Vector Structure") (Teleport :type Boolean))
  (`SceneComponent.K2_SetWorldLocation` (`self.StaticMesh`) Location false Teleport))

(event `self.AddImpulse`
  (params (Force :type "Vector Structure"))
  (`PrimitiveComponent.AddImpulse` (`self.StaticMesh`) Force "None" true))

(fn `GetLocation`
  (returns (NewParam :type "Vector Structure"))
  (return (`SceneComponent.K2_GetComponentLocation` (`self.StaticMesh`))))

(fn `UserConstructionScript`
  (`parent.UserConstructionScript`))