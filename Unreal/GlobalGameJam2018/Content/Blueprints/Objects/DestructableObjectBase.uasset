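; Base Blueprint for a floatable physics object that breaks when struck hard enough by other ObjectBase actors.
; An overlap box records the incoming object's speed, and on hit, while not floating, that speed times its weight is tested against this object's weight.
; Qualifying hits decrement hitpoints, or fracture the Destructible once they drop below one.
; Float, force and location overrides act on the Destructible, with floating disabling gravity and showing a Plane.
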(event `self.ReceiveBeginPlay`
  (`parent.ReceiveBeginPlay`)
  (set `self.PlaneOffset` (- (`SceneComponent.K2_GetComponentLocation` (`self.Plane`)) (`SceneComponent.K2_GetComponentLocation` (`self.Destructible`)))))

(event `self.ReceiveTick`
  (params (DeltaSeconds :type "Float (single-precision)"))
  (`parent.ReceiveTick` DeltaSeconds)
  (if (`self.IsFloating`)
    (`PrimitiveComponent.SetSimulatePhysics` (`self.Destructible`) true)))

(event `self.Destructible.OnComponentHit`
  (params (HitComponent :type "PrimitiveComponent Object Reference") (OtherActor :type "Actor Object Reference") (OtherComp :type "PrimitiveComponent Object Reference") (NormalImpulse :type "Vector Structure") (Hit :type "HitResult Structure (by ref)"))
  (bind _destructible (`self.Destructible`))
  (bind _othervelocity (`self.OtherVelocity`))
  (`KismetSystemLibrary.PrintString` "Actually insane")
  (if (`self.IsFloating`)
    (`KismetSystemLibrary.PrintString` "huh")
    (elif (`KismetMathLibrary.ClassIsChildOf` (`GameplayStatics.GetObjectClass` OtherActor) "/Game/Blueprints/Objects/ObjectBase.ObjectBase_C")
      (bind _asobject_base (cast `/Game/Blueprints/Objects/ObjectBase` OtherActor)
        (:`then`
          (`KismetSystemLibrary.PrintString` (`KismetStringLibrary.Conv_DoubleToString` _othervelocity))
          (bind _returnvalue (* _othervelocity (`/Game/Blueprints/Objects/ObjectBase.WeightLevel` _asobject_base)))
          (if (> _returnvalue (`self.WeightLevel`))
            (if (< (`self.Hitpoints`) 1.0)
              (`DestructibleComponent.ApplyDamage` _destructible 500.0 (`SceneComponent.K2_GetComponentLocation` _destructible) (0.0 0.0 1.0) _returnvalue)
              (else
                (bind _result (`/Engine/EditorBlueprintResources/StandardMacros.DecrementFloat` (`self.Hitpoints`))
                  (:`  `
                    (set `self.Hitpoints` _result)))))
            (else
              (`KismetSystemLibrary.PrintString` "Kong  Strong"))))
        (:`CastFailed`
          (`KismetSystemLibrary.PrintString` "Failed cast"))))))

(event `self.Box_0.OnComponentBeginOverlap`
  (params (OverlappedComponent :type "PrimitiveComponent Object Reference") (OtherActor :type "Actor Object Reference") (OtherComp :type "PrimitiveComponent Object Reference") (OtherBodyIndex :type Integer) (bFromSweep :type Boolean) (SweepResult :type "HitResult Structure (by ref)"))
  (bind _asobject_base (cast `/Game/Blueprints/Objects/ObjectBase` OtherActor))
  (`KismetSystemLibrary.PrintString` "getting vel")
  (if (`self.IsFloating`)
    (`KismetSystemLibrary.PrintString` "sfdsg")
    (elif (`KismetMathLibrary.ClassIsChildOf` (`GameplayStatics.GetObjectClass` OtherActor) "/Game/Blueprints/Objects/ObjectBase.ObjectBase_C")
      (bind _returnvalue (`KismetMathLibrary.VSize` (`/Game/Blueprints/Objects/ObjectBase.curvel` _asobject_base)))
      (set `self.OtherVelocity` _returnvalue)
      (`KismetSystemLibrary.PrintString` (`KismetStringLibrary.Conv_DoubleToString` _returnvalue)))))

(event `self.Float`
  (`parent.Float`)
  (`PrimitiveComponent.SetEnableGravity` (`self.Destructible`) false)
  (`SceneComponent.SetVisibility` (`self.Plane`) true false))

(event `self.StopFloat`
  (`parent.StopFloat`)
  (`PrimitiveComponent.SetEnableGravity` (`self.Destructible`) true)
  (`SceneComponent.SetVisibility` (`self.Plane`) false false))

(event `self.AddForceCustom`
  (params (Force :type "Vector Structure"))
  (`PrimitiveComponent.AddForce` (`self.Destructible`) Force "None" false))

(event `self.SetLocation`
  (params (Location :type "Vector Structure") (Teleport :type Boolean))
  (`SceneComponent.K2_SetWorldLocation` (`self.Destructible`) Location false Teleport))

(event `self.AddImpulse`
  (params (Force :type "Vector Structure"))
  (`PrimitiveComponent.AddImpulse` (`self.Destructible`) Force "None" false))

(fn `GetLocation`
  (returns (NewParam :type "Vector Structure"))
  (return (`SceneComponent.K2_GetComponentLocation` (`self.Destructible`))))

(fn `GetVel`
  (returns (NewParam :type "Vector Structure"))
  (bind _returnvalue (`PrimitiveComponent.GetPhysicsLinearVelocity` (`self.Destructible`) "None"))
  (return _returnvalue))

(fn `UserConstructionScript`
  (`parent.UserConstructionScript`))